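; Flapman is a physics-driven, flappy-style character whose Capsule is moved by velocity resets and forces.
; Each Jump press zeroes the capsule's velocity and applies an upward force, giving a consistent flap.
; While the capsule rises, Tick adds downforce unless the Jump value reads fully held, so releasing early cuts the flap short for variable jump height.
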(event EventBeginPlay)

(event Collision|EventActorBeginOverlap
  (params (OtherActor :type Actor%20Object%20Reference)))

(event EventTick
  (params (DeltaSeconds :type Float%20%28single-precision%29))
  (bind _returnvalue (Physics|GetPhysicsLinearVelocity (Variables|Components|GetCapsule) "None"))
  (if (> (.z _returnvalue) 0.0)
    (if (== (Input|AxisValues|GetJump) 1.0)
      (Variables|Default|SetDownforce 0.0)
      (else
        (Variables|Default|SetDownforce -1e+04)))
    (Physics|AddForce (Variables|Components|GetCapsule) (Math|Vector|MakeVector 0.0 0.0 (Variables|Default|GetDownforce)) "None" false)))

(event Input|ActionEvents|InputActionJump
  (params (Key :type Key%20Structure :default "None"))
  (:Pressed
    (Physics|SetPhysicsLinearVelocity (Variables|Components|GetCapsule) "0, 0, 0" false "None")
    (Physics|AddForce (Variables|Components|GetCapsule) "0, 0,30000.000000" "None" false)))

(fn ConstructionScript)