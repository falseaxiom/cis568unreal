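; Block is an actor that moves steadily along world X while bobbing vertically.
; On BeginPlay it shifts its root component by a random Z offset.
; Each Tick advances X at a constant speed scaled by delta time and sets Z to an absolute sine of game time, which overwrites the random starting height.
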(event EventBeginPlay
  (Transformation|SetWorldLocation (Variables|Default|GetDefaultSceneRoot) (+ (Transformation|GetWorldLocation (Variables|Default|GetDefaultSceneRoot)) (Math|Vector|MakeVector 0.0 0.0 (Math|Random|RandomFloatinRange -3e+02 3e+02))) false false))

(event Collision|EventActorBeginOverlap
  (params (OtherActor :type Actor%20Object%20Reference)))

(event EventTick
  (params (DeltaSeconds :type Float%20%28single-precision%29))
  (bind _returnvalue (Math|Float|MakeLiteralFloat 5e+02))
  (bind _defaultsceneroot (Variables|Default|GetDefaultSceneRoot))
  (bind _returnvalue_2 (Transformation|GetWorldLocation _defaultsceneroot))
  (bind _returnvalue_3 (* DeltaSeconds _returnvalue))
  (bind _returnvalue_4 (Math|Vector|MakeVector _returnvalue_3 0.0 0.0))
  (bind _returnvalue_5 (+ _returnvalue_2 _returnvalue_4))
  (Transformation|SetWorldLocation (Variables|Default|GetDefaultSceneRoot) (Math|Vector|MakeVector (.x _returnvalue_5) (.y _returnvalue_5) (* (Math|Trig|Sin(Radians) (Utilities|Time|GetGameTimeinSeconds)) (Math|Float|MakeLiteralFloat 1e+02))) false false))

(fn ConstructionScript)